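; BP_DoubleJumpPowerUp is a Platforms2D pickup that unlocks double jump for the player's SwatCharacter.
; On BeginPlay it loads the save using the game instance's slot name and user index, and destroys itself if the saved max jump count already allows a double jump.
; On overlap with a BP_SwatCharacter it calls UnlockDoubleJump on that character, then destroys itself.
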(event EventBeginPlay
  (bind _asbp_platforms_2dgame_instance (Utilities|Casting|CastToBP_Platforms2DGameInstance (Game|GetGameInstance)))
  (bind _returnvalue (SaveGame|DoesSaveGameExist (Variables|/Game/Platforms2D/Blueprints/BP_Platforms2DGameInstance.BP_Platforms2DGameInstance_C|GetSaveSlotName _asbp_platforms_2dgame_instance) (Variables|/Game/Platforms2D/Blueprints/BP_Platforms2DGameInstance.BP_Platforms2DGameInstance_C|GetUserIndex _asbp_platforms_2dgame_instance)))
  (if _returnvalue
    (bind _returnvalue_2 (SaveGame|LoadGamefromSlot (Variables|/Game/Platforms2D/Blueprints/BP_Platforms2DGameInstance.BP_Platforms2DGameInstance_C|GetSaveSlotName _asbp_platforms_2dgame_instance) (Variables|/Game/Platforms2D/Blueprints/BP_Platforms2DGameInstance.BP_Platforms2DGameInstance_C|GetUserIndex _asbp_platforms_2dgame_instance)))
    (bind _asbp_platforms_2dsave_game (Utilities|Casting|CastToBP_Platforms2DSaveGame _returnvalue_2))
    (if (>= (Variables|/Game/Platforms2D/Blueprints/SaveGame/BP_Platforms2DSaveGame.BP_Platforms2DSaveGame_C|GetJumpMaxCount _asbp_platforms_2dsave_game) 2)
      (Actor|DestroyActor))))

(event Collision|EventActorBeginOverlap
  (params (OtherActor :type Actor%20Object%20Reference))
  (bind _asbp_swat_character (Utilities|Casting|CastToBP_SwatCharacter OtherActor))
  (Default|UnlockDoubleJump _asbp_swat_character)
  (Actor|DestroyActor))

(fn ConstructionScript)