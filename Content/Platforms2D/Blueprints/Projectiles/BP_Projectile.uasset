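; Projectile actor for the 2D platformer that flies at a configurable speed and damages what it hits.
; The construction script copies Speed into the projectile movement component's initial speed, and a BeginPlay timer destroys the actor when its Lifetime expires.
; Overlapping any actor not tagged IgnoreProjectile spawns an explosion effect and sound, applies damage of the set type, then clears the timer and destroys the projectile.
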(event Custom|LifetimeEnds
  ;[0 0 0] Lifetime Event Ends
  (Actor|DestroyActor))

(event EventBeginPlay
  ;[0 0 0] Lifetime Event
  (bind _returnvalue (Utilities|Time|SetTimerbyEvent (delegate Custom|LifetimeEnds) (Variables|ProjectileCustom|GetLifetime)))
  (Variables|Events|SetLifetimeEventEnds _returnvalue))

(event Collision|EventActorBeginOverlap
  (params (OtherActor :type Actor%20Object%20Reference))
  (bind _returnvalue (Transformation|GetActorLocation))
  (if (not (Actor|ActorHasTag OtherActor "IgnoreProjectile"))
    (Utilities|FlowControl|Sequence
      (:then_0
        ;[0 0 0] Spawn FX
        (Effects|SpawnEmitteratLocation "/Game/StarterContent/Particles/P_Explosion.P_Explosion" _returnvalue "0, 0, 0" "0.500000,0.500000,0.500000")
        (Audio|PlaySoundatLocation "/Game/StarterContent/Audio/Explosion01.Explosion01" _returnvalue "0, 0, 0" 0.075 1.0 0.0 0 0 0 0))
      (:then_1
        ;[0 0 0] Damage
        (Game|Damage|ApplyDamage OtherActor (Variables|ProjectileCustom|GetDamage) 0 0 "/Script/Engine.DamageType"))
      (:then_2
        ;[0 0 0] Destroy
        (Utilities|Time|ClearandInvalidateTimerbyHandle (Variables|Events|GetLifetimeEventEnds))
        (Actor|DestroyActor)))))

(fn ConstructionScript
  (Variables|/Script/Engine.ProjectileMovementComponent|SetInitialSpeed (Variables|Default|GetProjectileMovementComponent) (Variables|ProjectileCustom|GetSpeed)))