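; BP_Wall is a movable wall for the 2D platforms game that slides to a target position once activated.
; Activate sets the StartMovement flag, and Tick then interpolates the Cube's world location toward the Arrow component's location with VInterpTo.
; The Arrow serves as the destination marker, and the move runs without sweep, with no stop or reset logic.
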(event EventTick
  (params (DeltaSeconds :type Float%20%28single-precision%29))
  (if (Variables|Default|GetStartMovement)
    (Transformation|SetWorldLocation (Variables|Default|GetCube) (Math|Interpolation|VInterpTo (Transformation|GetWorldLocation (Variables|Default|GetCube)) (Transformation|GetWorldLocation (Variables|Default|GetArrow)) DeltaSeconds 25.0) false false)))

(fn ConstructionScript)

(fn Activate
  (Variables|Default|SetStartMovement true))