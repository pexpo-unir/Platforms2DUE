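; Turret actor for the 2D platform game that spawns projectiles at its muzzle and can be destroyed by damage.
; While IsActive, Tick calls Fire, which spawns the configured projectile class and gates repeat shots with a one-shot cooldown timer.
; Any damage taken lowers Health, updates the BP_3DHealthBar widget and destroys the actor once health runs out.
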(event Custom|EventFireCooldownFinish
  (Variables|Turret|SetCanFireProjectile true))

(event Custom|OnTakeAnyDamage_Event
  (params (DamagedActor :type Actor%20Object%20Reference) (Damage :type Float%20%28single-precision%29) (DamageType :type Damage%20Type%20Object%20Reference) (InstigatedBy :type Controller%20Object%20Reference) (DamageCauser :type Actor%20Object%20Reference))
  ;[0 0 0] Take Damage
  (bind _output_get (Variables|Health|SetHealth (- (Variables|Health|GetHealth) Damage)))
  (bind _asbp_3dhealth_bar (Utilities|Casting|CastToBP_3DHealthBar (UserInterface|GetWidget (Variables|Default|GetWidget))))
  (Default|UpdateHealth _asbp_3dhealth_bar _output_get)
  ;[1 0 0] Check if dead
  (if (<= (Variables|Health|GetHealth) 0.0)
    (Actor|DestroyActor)))

(event EventBeginPlay
  ;[0 0 0] Take Damage
  (EventDispatchers|BindEventtoOnTakeAnyDamage (delegate Custom|OnTakeAnyDamage_Event))
  (bind _asbp_3dhealth_bar (Utilities|Casting|CastToBP_3DHealthBar (UserInterface|GetWidget (Variables|Default|GetWidget))))
  (Default|UpdateHealth _asbp_3dhealth_bar (stale Custom|OnTakeAnyDamage_Event _output_get))
  ;[1 0 0] Check if dead
  (if (<= (Variables|Health|GetHealth) 0.0)
    (Actor|DestroyActor)))

(event EventTick
  (params (DeltaSeconds :type Float%20%28single-precision%29))
  (if (Variables|Turret|GetIsActive)
    (CallFunction|Fire)))

(fn ConstructionScript)

(fn Fire
  (if (Variables|Turret|GetCanFireProjectile)
    (Utilities|Time|SetTimerbyEvent (EventDispatchers|CreateEvent :!event Custom|EventFireCooldownFinish) (Variables|Turret|GetFireProjectileCooldown))
    (Variables|Turret|SetCanFireProjectile false)
    (bind _projectileclass (Variables|Turret|GetProjectileClass)
      (:then
        (Game|SpawnActorfromClass _projectileclass (Transformation|GetWorldTransform (Variables|Default|GetMuzzle)) "Undefined" "MultiplyWithRoot" 0 0))
      (:else))))